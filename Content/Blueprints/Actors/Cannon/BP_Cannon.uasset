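; BP_Cannon is an actor that automatically fires projectiles in an endless loop from BeginPlay.
; After a ShootingSpeed delay, it spawns a BP_Projectile at the Arrow component's location and rotation, scaled by ProjectileScale.
; The CannonLocation timeline then animates the Cannon component's relative Y position through CannonAnimation, and its completion restarts the delay for the next shot.
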(event Collision|EventActorBeginOverlap
  (params (OtherActor :type Actor%20Object%20Reference)))

(event EventBeginPlay
  (bind _arrow (Variables|Default|GetArrow))
  (Utilities|FlowControl|Delay (Variables|CannonProperties|GetShootingSpeed) :!label _label)
  (Game|SpawnActorfromClass "/Game/Blueprints/Actors/Projectiles/BP_Projectile.BP_Projectile_C" (Math|Transform|MakeTransform (Transformation|GetWorldLocation _arrow) (Transformation|GetWorldRotation _arrow) (Math|Conversions|ToVector(Float) (Variables|ProjectileProperties|GetProjectileScale))) "Undefined" 0 0)
  (bind _cannonchangey (Timeline|CannonLocation PlayFromStart)
    (:Update
      (CallFunction|CannonAnimation _cannonchangey))
    (:Finished
      (goto _label))))

(fn ConstructionScript)

(fn CannonAnimation
  (params (NewLocation_Y :type Float%20%28single-precision%29))
  (Transformation|SetRelativeLocation (Variables|Default|GetCannon) (Math|Vector|MakeVector 0.0 NewLocation_Y 0.0) false false))