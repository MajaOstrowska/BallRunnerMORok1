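; BP_WinVolume is a level exit trigger that lets the player advance once every crystal is collected.
; On box overlap by the player, it counts remaining BP_Object actors, treating none left as all crystals collected.
; Success prints a Polish message and opens the hard-coded Level_02 after a short delay; otherwise it prints a not-all-collected message.
; LevelList-based progression and quit-on-last-level logic exists but is disconnected.
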(event OnComponentBeginOverlap(Box)
  (params (OverlappedComponent :type Primitive%20Component%20Object%20Reference) (OtherActor :type Actor%20Object%20Reference) (OtherComp :type Primitive%20Component%20Object%20Reference) (OtherBodyIndex :type Integer) (bFromSweep :type Boolean) (SweepResult :type Hit%20Result%20Structure%20%28by%20ref%29))
  (Utilities|IsPlayer OtherActor OtherActor
    (:True
      (if (CallFunction|CheckAllCrystals)
        (Development|PrintString "Zebrales wszytskie krysztaly")
        (Utilities|FlowControl|Delay 0.2)
        (Game|OpenLevel(byName) "Level_02")
        (else
          (Development|PrintString "Nie zebrales wszytskich krysztalow"))))))

(fn ConstructionScript)

(fn CheckAllCrystals
  (bind _outactors (Actor|GetAllActorsOfClass "/Game/Blueprints/Actors/Collectables/BP_Object.BP_Object_C"))
  (return (== (Utilities|Array|Length _outactors) 0)))

(fn CheckCurrentIndex
  (bind _returnvalue (Game|GetCurrentLevelName true))
  (return (Utilities|Array|FindItem (Variables|Default|GetLevelList) (Utilities|String|StringToName _returnvalue))))