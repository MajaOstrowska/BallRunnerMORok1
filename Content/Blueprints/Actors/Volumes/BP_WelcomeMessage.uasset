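; Welcome trigger volume that shows a one-time message sequence with confetti when the player first overlaps its box.
; DoOnce gates a sequence: welcome text, confetti emitter at the actor's location, short delay, then the restart and exit messages in turn.
; Each message sub-graph toggles its component's visibility, waits a second, then toggles it back.
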(event OnComponentBeginOverlap(Box)
  (params (OverlappedComponent :type Primitive%20Component%20Object%20Reference) (OtherActor :type Actor%20Object%20Reference) (OtherComp :type Primitive%20Component%20Object%20Reference) (OtherBodyIndex :type Integer) (bFromSweep :type Boolean) (SweepResult :type Hit%20Result%20Structure%20%28by%20ref%29))
  (Utilities|IsPlayer OtherActor
    (:True
      (Utilities|FlowControl|DoOnce false
        (:Completed
          (Utilities|WelcomeText)
          (Effects|SpawnEmitteratLocation "/Game/Particles/P_Confetti.P_Confetti" (Transformation|GetActorLocation))
          (Utilities|FlowControl|Delay 0.2)
          (Utilities|RestartMessage)
          (Utilities|Quitmessage))))))

(event EventBeginPlay)

(event Collision|EventActorBeginOverlap
  (params (OtherActor :type Actor%20Object%20Reference)))

(event EventTick
  (params (DeltaSeconds :type Float%20%28single-precision%29)))

(fn ConstructionScript)