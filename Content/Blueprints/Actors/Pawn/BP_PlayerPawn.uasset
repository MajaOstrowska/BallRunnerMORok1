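; BP_PlayerPawn is a physics-driven player pawn that moves by applying torque to its static mesh.
; Forward/backward and right/left axis inputs scale by Multipy into acceleration-based torque on the Y and X axes.
; Any damage calls FadeRestart, whose body is not shown here.
; Helper functions fade the camera out, and start a fade-in while calling OpenLevelByName with an empty name.
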(event EventBeginPlay)

(event Collision|EventActorBeginOverlap
  (params (OtherActor :type Actor%20Object%20Reference)))

(event EventTick
  (params (DeltaSeconds :type Float%20%28single-precision%29)))

(event Game|Damage|EventAnyDamage
  (params (Damage :type Float%20%28single-precision%29) (DamageType :type Damage%20Type%20Object%20Reference) (InstigatedBy :type Controller%20Object%20Reference) (DamageCauser :type Actor%20Object%20Reference))
  (Utilities|Fade&Restart))

(event Input|AxisEvents|InputAxisMoveForewards/Backwards
  (params (AxisValue :type Float%20%28single-precision%29))
  (Class|PrimitiveComponent|AddTorqueinRadians (Variables|Default|GetStaticMesh) (Math|Vector|MakeVector 0.0 (* AxisValue (Variables|BallVariables|GetMultipy)) 0.0) "None" true))

(event Input|AxisEvents|InputAxisMoveRight/Left
  (params (AxisValue :type Float%20%28single-precision%29))
  (Class|PrimitiveComponent|AddTorqueinRadians (Variables|Default|GetStaticMesh) (Math|Vector|MakeVector (* AxisValue (Variables|BallVariables|GetMultipy)) 0.0 0.0) "None" true))

(fn ConstructionScript)

(fn OpenLevel
  (params (Duration :type Float%20%28single-precision%29))
  (CameraFades|StartCameraFade :self (Game|GetPlayerCameraManager 0) :FromAlpha 1.0 :Duration Duration)
  (Game|OpenLevel(byName) (Utilities|String|StringToName "")))

(fn CameraFade
  (bind _returnvalue (Math|Float|MakeLiteralFloat 1.0))
  (CameraFades|StartCameraFade :self (Game|GetPlayerCameraManager 0) :ToAlpha 1.0 :Duration _returnvalue)
  (return _returnvalue))