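; BP_Object is a collectable crystal that flies into the player when touched, then destroys itself.
; A player overlap on the Sphere caches the actor's location, scale and PointLight intensity, then plays the TL_BlendAlpha timeline.
; Separate timeline tracks drive lerps toward the player pawn's current position, zero scale and zero light, so the crystal homes in as it shrinks and dims.
; No score or inventory update happens here.
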(event OnComponentBeginOverlap(Sphere)
  (params (OverlappedComponent :type Primitive%20Component%20Object%20Reference) (OtherActor :type Actor%20Object%20Reference) (OtherComp :type Primitive%20Component%20Object%20Reference) (OtherBodyIndex :type Integer) (bFromSweep :type Boolean) (SweepResult :type Hit%20Result%20Structure%20%28by%20ref%29))
  (Utilities|IsPlayer OtherActor
    (:True
      (CallFunction|CrystalProperties)
      (bind (_direction _smoothlerpalpha _lerpscale _lerplight) (Timeline|TL_BlendAlpha Play)
        (:Update
          (CallFunction|LerpLocation _smoothlerpalpha)
          (CallFunction|LerpScale _lerpscale)
          (CallFunction|LerpLight _lerplight))
        (:Finished
          (Actor|DestroyActor))))))

(event EventBeginPlay)

(event EventTick
  (params (DeltaSeconds :type Float%20%28single-precision%29)))

(fn ConstructionScript)

(fn LerpScale
  (params (Alpha :type Float%20%28single-precision%29))
  (Transformation|SetActorScale3D (Math|Vector|Lerp(Vector) (Variables|Default|GetCrystalScale) "0, 0, 0" Alpha)))

(fn LerpLight
  (params (Alpha :type Float%20%28single-precision%29))
  (Rendering|Components|Light|SetIntensity (Variables|Default|GetPointLight) (Math|Float|Lerp (Variables|Default|GetCrystalIntensity) 0.0 Alpha)))

(fn CrystalProperties
  (Variables|Default|SetCrystalLocation (Transformation|GetActorLocation))
  (Variables|Default|SetCrystalScale (Transformation|GetActorScale3D))
  (Variables|Default|SetCrystalIntensity (Variables|/Script/Engine.LightComponentBase|GetIntensity (Variables|Default|GetPointLight))))

(fn LerpLocation
  (params (Alpha :type Float%20%28single-precision%29))
  (Transformation|SetActorLocation (Math|Vector|Lerp(Vector) (Variables|Default|GetCrystalLocation) (Transformation|GetActorLocation (Game|Player|GetPlayerPawn 0)) Alpha) false false))